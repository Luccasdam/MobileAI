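; AI character Blueprint that shows a state label above or on itself through an animated text render component.
; DisplayState takes a struct, sets the text and timeline play rate, then makes the text visible and starts the timeline, which scales its world size up from zero.
; After each finish and a display-time delay, looping states alternate between shrinking and growing, while others hide the text and stop the timeline.
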(event Custom|ReverseDisplayText
  ;[1 1 1] Display State Text
  (bind (_direction _alpha) (Timeline|Timeline_DisplayStateText ReverseFromEnd)
    (:Update
      (Rendering|Components|TextRender|SetWorldSize (Variables|Default|GetTextRenderComp) (Math|Float|Lerp 0.0 1e+02 _alpha)))
    (:Finished
      (Utilities|FlowControl|Delay (.DisplayTime (Utilities|Struct|BreakDisplayStateStruct (stale EventDisplayState DisplayStateStruct))))
      (if (.bLoop (Utilities|Struct|BreakDisplayStateStruct (stale EventDisplayState DisplayStateStruct)))
        (if (Utilities|Enum|Equal(Enum) _direction "Forward")
          (CallFunction|ReverseDisplayText)
          (else
            (CallFunction|PlayDisplayText)))
        (else
          (Class|MAICharacter|StopDisplayState))))))

(event Custom|PlayDisplayText
  ;[1 1 1] Display State Text
  (bind (_direction _alpha) (Timeline|Timeline_DisplayStateText PlayFromStart)
    (:Update
      (Rendering|Components|TextRender|SetWorldSize (Variables|Default|GetTextRenderComp) (Math|Float|Lerp 0.0 1e+02 _alpha)))
    (:Finished
      (Utilities|FlowControl|Delay (.DisplayTime (Utilities|Struct|BreakDisplayStateStruct (stale EventDisplayState DisplayStateStruct))))
      (if (.bLoop (Utilities|Struct|BreakDisplayStateStruct (stale EventDisplayState DisplayStateStruct)))
        (if (Utilities|Enum|Equal(Enum) _direction "Forward")
          (CallFunction|ReverseDisplayText)
          (else
            (CallFunction|PlayDisplayText)))
        (else
          (Class|MAICharacter|StopDisplayState))))))

(event EventDisplayState
  (params (DisplayStateStruct :type Display%20State%20Struct%20Structure))
  (bind (_displaytext _playrate _displaytime _bloop) (Utilities|Struct|BreakDisplayStateStruct DisplayStateStruct))
  ;[1 1 1] Display State Text
  (Rendering|Components|TextRender|SetText (Variables|Default|GetTextRenderComp) (Utilities|Text|ToText(String) _displaytext))
  (Components|Timeline|SetPlayRate (Variables|Default|GetTimeline_DisplayStateText) _playrate)
  (Rendering|Components|TextRender|SetWorldSize (Variables|Default|GetTextRenderComp) 0.0)
  (Rendering|SetVisibility (Variables|Default|GetTextRenderComp) true false)
  (bind (_direction _alpha) (Timeline|Timeline_DisplayStateText PlayFromStart)
    (:Update
      (Rendering|Components|TextRender|SetWorldSize (Variables|Default|GetTextRenderComp) (Math|Float|Lerp 0.0 1e+02 _alpha)))
    (:Finished
      (Utilities|FlowControl|Delay _displaytime)
      (if _bloop
        (if (Utilities|Enum|Equal(Enum) _direction "Forward")
          (CallFunction|ReverseDisplayText)
          (else
            (CallFunction|PlayDisplayText)))
        (else
          (Class|MAICharacter|StopDisplayState))))))

(event EventStopDisplayState
  ;[1 1 1] Display State Text
  (Rendering|SetVisibility (Variables|Default|GetTextRenderComp) false false)
  (bind (_direction _alpha) (Timeline|Timeline_DisplayStateText Stop)
    (:Update
      (Rendering|Components|TextRender|SetWorldSize (Variables|Default|GetTextRenderComp) (Math|Float|Lerp 0.0 1e+02 _alpha)))
    (:Finished
      (Utilities|FlowControl|Delay (.DisplayTime (Utilities|Struct|BreakDisplayStateStruct (stale EventDisplayState DisplayStateStruct))))
      (if (.bLoop (Utilities|Struct|BreakDisplayStateStruct (stale EventDisplayState DisplayStateStruct)))
        (if (Utilities|Enum|Equal(Enum) _direction "Forward")
          (CallFunction|ReverseDisplayText)
          (else
            (CallFunction|PlayDisplayText)))
        (else
          (Class|MAICharacter|StopDisplayState))))))

(fn ConstructionScript)